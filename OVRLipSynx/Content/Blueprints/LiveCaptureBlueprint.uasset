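; Live capture Blueprint that lip-syncs a skeletal mesh using an OVRLipSync component.
; It starts OVRLipSync on BeginPlay and, on Windows, zeroes the mic threshold and voice noise gate to disable silence detection.
; Whenever visemes are ready, it assigns them to the mesh's morph targets and drives a "laughter" morph from the remapped, clamped laughter score.
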(event OnVisemesReady(OVRLipSync)
  (bind _skeletalmeshcomponent (Variables|SkeletalMeshActor|GetSkeletalMeshComponent))
  (bind _ovrlipsync (Variables|Default|GetOVRLipSync))
  (Class|OVRLipSyncActorComponentBase|AssignVisemestoMorphTargets _ovrlipsync _skeletalmeshcomponent)
  (Components|SkeletalMesh|SetMorphTarget _skeletalmeshcomponent "laughter" (Math|Float|MapRangeClamped (Class|OVRLipSyncActorComponent|GetLaughterScore _ovrlipsync) 0.4 1.0 0.0 1.0) true))

(event EventBeginPlay
  (Class|OVRLipSyncActorComponent|Start (Variables|Default|GetOVRLipSync))
  ;[1 1 1] Disable silence detection on Windows
  (if (Utilities|String|Contains (Game|GetPlatformName) "Win")
    (Class|VOIPStatics|SetMicThreshold 0.0)
    (Development|ExecuteConsoleCommand "voice.MicNoiseGateThreshold 0.0" 0)))

(fn ConstructionScript)